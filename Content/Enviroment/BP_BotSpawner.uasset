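; BP_BotSpawner is a team-tagged marker actor for bot spawn points, though it contains no spawning logic itself.
; The construction script colors its Cube blue or red from TeamID and adds a small rotated arrow component at each relative Points entry, collecting them in Arrows.
; BeginPlay only prints each arrow's world location on screen for a long duration, as debug output.
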(event EventBeginPlay
  (for _array_element (Variables|Default|GetArrows)
    (Development|PrintString (Utilities|String|ToString(Vector) (Transformation|GetWorldLocation _array_element)) true true "(R=0.000000,G=0.660000,B=1.000000,A=1.000000)" 4646.0)))

(event Collision|EventActorBeginOverlap
  (params (OtherActor :type Actor%20Object%20Reference)))

(event EventTick
  (params (DeltaSeconds :type Float%20%28single-precision%29)))

(fn ConstructionScript
  (bind _cube (Variables|Default|GetCube))
  (switch int (Variables|Default|GetTeamID)
    (:1
      (Rendering|Material|SetMaterial _cube 0 "/Game/Materials/M_Blue.M_Blue"))
    (:2
      (Rendering|Material|SetMaterial _cube 0 "/Game/Materials/M_Red.M_Red")))
  (for _array_element (Variables|Default|Getpoints)
    (bind _returnvalue (AddComponent|AddArrowComponent false (Math|Transform|MakeTransform _array_element "90.000000,90.000000,0.000000" "0.500000,0.500000,0.500000")))
    (Utilities|Array|Add (Variables|Default|GetArrows) _returnvalue)))