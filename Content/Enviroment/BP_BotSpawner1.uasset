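; BP_BotSpawner1 is a team-colored spawner that spawns one BP_STUPlayerCharacter at a randomly chosen point on BeginPlay.
; It collects five scene components into an array and uses a random element's world location as the spawn transform.
; A debug print shows a separately randomized location, so it can differ from the actual spawn point.
; The construction script colors the cube blue or red from TeamID, which is not passed to the spawned character.
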(event EventBeginPlay
  (bind _ui_jopa (Variables|Default|Getui_jopa))
  (bind _outitem (Utilities|Array|Random _ui_jopa))
  (bind _returnvalue (Transformation|GetWorldLocation _outitem))
  (Utilities|Array|Add (Variables|Default|Getui_jopa) (Variables|Default|GetScene))
  (Utilities|Array|Add (Variables|Default|Getui_jopa) (Variables|Default|GetScene1))
  (Utilities|Array|Add (Variables|Default|Getui_jopa) (Variables|Default|GetScene2))
  (Utilities|Array|Add (Variables|Default|Getui_jopa) (Variables|Default|GetScene3))
  (Utilities|Array|Add (Variables|Default|Getui_jopa) (Variables|Default|GetScene4))
  (Development|PrintString (Utilities|String|ToString(Vector) _returnvalue) true true "(R=0.000000,G=0.660000,B=1.000000,A=1.000000)" 999.0)
  (Game|SpawnActorfromClass "/Game/Player/BP_STUPlayerCharacter.BP_STUPlayerCharacter_C" (Math|Conversions|ToTransform(Vector) _returnvalue) "Undefined" 0 0))

(event Collision|EventActorBeginOverlap
  (params (OtherActor :type Actor%20Object%20Reference)))

(event EventTick
  (params (DeltaSeconds :type Float%20%28single-precision%29)))

(fn ConstructionScript
  (bind _cube (Variables|Default|GetCube))
  (switch int (Variables|Default|GetTeamID)
    (:1
      (Rendering|Material|SetMaterial _cube 0 "/Game/Materials/M_Blue.M_Blue"))
    (:2
      (Rendering|Material|SetMaterial _cube 0 "/Game/Materials/M_Red.M_Red"))))