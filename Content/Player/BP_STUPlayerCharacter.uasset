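; Player character Blueprint that adds two debug-style key bindings, with empty BeginPlay and construction script.
; Tab press and release pass a held-state boolean to Shesh on BP_STUGameHUD, found by searching all actors of the game mode's HUD class.
; X creates a dynamic material instance on the mesh's first material slot and sets its Paint Color to pink.
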(event EventBeginPlay)

(event Collision|EventActorBeginOverlap
  (params (OtherActor :type Actor%20Object%20Reference)))

(event EventTick
  (params (DeltaSeconds :type Float%20%28single-precision%29)))

(event Input|KeyboardEvents|Tab
  (params (Key :type Key%20Structure :default "None"))
  (:Pressed
    (Variables|Default|SetPressed true)
    (bind _outactors (Actor|GetAllActorsOfClass (Variables|/Script/Engine.GameModeBase|GetHUDClass (Game|GetGameMode)) :!label _label))
    (bind _asbp_stugame_hud (Utilities|Casting|CastToBP_STUGameHUD (Utilities|Array|Get(acopy) _outactors)))
    (Default|Shesh _asbp_stugame_hud (Variables|Default|GetPressed)))
  (:Released
    (Variables|Default|SetPressed false)
    (goto _label)))

(event Input|KeyboardEvents|X
  (params (Key :type Key%20Structure :default "None"))
  (:Pressed
    (bind _returnvalue (Rendering|Material|CreateDynamicMaterialInstance (Variables|Character|GetMesh) 0 0 "None" :!class /Script/Engine.PrimitiveComponent))
    (Rendering|Material|SetVectorParameterValue _returnvalue "Paint Color" "(R=1.000000,G=0.535435,B=0.862750,A=1.000000)" :!class /Script/Engine.MaterialInstanceDynamic)))

(fn ConstructionScript)